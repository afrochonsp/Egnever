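; BP_NPC is an interactable NPC that shows an action selection menu when the player interacts with it.
; Interact stores the calling InteractComponent, shows the widget component and returns flags to stop interaction, disable input and show the cursor.
; On BeginPlay it binds to the WBP_ActionSelection exit event, which hides the menu, restores interaction on the stored component and clears the reference.
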(event `self.ReceiveBeginPlay`
  (`parent.ReceiveBeginPlay`)
  (bind _aswbp_action_selection (cast `/Game/Blueprints/ActionSelecting/WBP_ActionSelection` (`WidgetComponent.GetWidget` (`self.Widget`))))
  (add `/Game/Blueprints/ActionSelecting/WBP_ActionSelection.OnExit` _aswbp_action_selection (`|CreateDelegate` :!event `OnMenuExit`)))

(event `OnMenuExit`
  (`SceneComponent.SetVisibility` (`self.Widget`) false false)
  (`/Game/Blueprints/Interaction/BP_InteractComponent.RestoreInteract` (`self.Interact Component`))
  (set `self.Interact Component` null))

(fn `CanInteract`
  (params (InteractComponent :type "/Game/Blueprints/Interaction/BP_InteractComponent Object Reference"))
  (returns (ReturnValue :type Boolean))
  (return true))

(fn `Interact`
  (params (InteractComponent :type "/Game/Blueprints/Interaction/BP_InteractComponent Object Reference"))
  (returns (StopInteraction :type Boolean) (DisableInput :type Boolean) (ShowCursor :type Boolean))
  (set `self.Interact Component` InteractComponent)
  (`SceneComponent.SetVisibility` (`self.Widget`) true false)
  (return true true true))

(fn `UserConstructionScript`
  (`parent.UserConstructionScript`))