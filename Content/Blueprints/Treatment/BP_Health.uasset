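; BP_Health tracks hit points for its owner and signals death or full restoration.
; It starts HP at the default capped by MaxHP, and AddHP and SubtractHP both route through SetHP.
; SetHP clamps between zero and the higher of MaxHP or current HP, then calls OnDeath at zero and OnRestored at exactly MaxHP, even if the value is unchanged.
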(event `self.ReceiveBeginPlay`
  (set `self.HP` (`KismetMathLibrary.Min` (`self.DefaultHP`) (`self.MaxHP`))))

(fn `AddHP`
  (params (Value :type Integer))
  (`self.SetHP` (`KismetMathLibrary.Max` (+ Value (`self.HP`)))))

(fn `GetHP`
  (returns (`Return Value` :type Integer))
  (return (`self.HP`)))

(fn `SetHP`
  (params (`New Value` :type Integer))
  (bind _output_get (set `self.HP` (`KismetMathLibrary.Clamp` `New Value` 0 (`KismetMathLibrary.Max` (`self.MaxHP`) (`self.HP`)))))
  (`|ExecutionSequence`
    (:`then_0`
      (if (== _output_get 0)
        (`self.OnDeath`)))
    (:`then_1`
      (if (== _output_get (`self.MaxHP`))
        (`self.OnRestored`)))))

(fn `SubtractHP`
  (params (Value :type Integer))
  (`self.AddHP` (* Value -1)))