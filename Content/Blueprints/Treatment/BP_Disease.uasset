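; Disease component that periodically makes its owner need treatment, shows a medicine widget and randomizes a three-drug dose recipe.
; TreatMixture requires an exact dose match; Treat adds or subtracts HP on the owner's BP_Health and hides the widget.
; Chained one-shot timers, pausable via Pause/Unpause, drive a randomly delayed onset and a damage deadline that penalizes untreated disease before rescheduling.
; The disease type is currently fixed, with random selection left unused.
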(event `self.ReceiveBeginPlay`
  (`self.StartDisease`))

(event `StartDisease`
  (bind _returnvalue (`KismetSystemLibrary.K2_SetTimerDelegate` (`|CreateDelegate` :!event `Disease`) (+ (`self.Delay`) (`KismetMathLibrary.RandomFloatInRange` 0.0 (`self.RandomOffset`)))))
  (set `self.DiseaseTimer` _returnvalue))

(event `Disease`
  (bind _mixturetreatment (`self.MixtureTreatment`))
  (bind _returnvalue (`KismetMathLibrary.Conv_IntToDouble` (* (`KismetMathLibrary.RandomIntegerInRange` 1 3) 10)))
  (set `self.bNeedTreatment` true)
  (set `self.bCanTreat` false)
  (set `self.CurrentDisease` "NewEnumerator2")
  (`BlueprintMapLibrary.Map_Add` _mixturetreatment "NewEnumerator0" _returnvalue)
  (`BlueprintMapLibrary.Map_Add` _mixturetreatment "NewEnumerator1" _returnvalue)
  (`BlueprintMapLibrary.Map_Add` _mixturetreatment "NewEnumerator2" _returnvalue)
  (`SceneComponent.SetVisibility` (`self.MedicineWidget`) true false)
  (bind _returnvalue_2 (`KismetSystemLibrary.K2_SetTimerDelegate` (`|CreateDelegate` :!event `DiseaseDamage`) (`self.DamageDelay`)))
  (set `self.DamageTimer` _returnvalue_2))

(event `DiseaseDamage`
  (if (`self.bNeedTreatment`)
    (`self.Treat` false))
  (`self.StartDisease`))

(fn `GetDisease`
  (returns (`Return Value` :type "/Game/Blueprints/Treatment/EDiseases Enum"))
  (return (`self.CurrentDisease`)))

(fn `IsNeedTreatment`
  (returns (`Return Value` :type Boolean))
  (return (`self.bNeedTreatment`)))

(fn `Pause`
  (`KismetSystemLibrary.K2_PauseTimerHandle` (`self.DiseaseTimer`))
  (`KismetSystemLibrary.K2_PauseTimerHandle` (`self.DamageTimer`)))

(fn `SetMedicineWidget`
  (params (`New Value` :type "WidgetComponent Object Reference"))
  (set `self.MedicineWidget` `New Value`))

(fn `Treat`
  (params (Success :type Boolean))
  (bind _damage (`self.Damage`))
  (bind _returnvalue (`Actor.GetComponentByClass` (`self.GetOwner`) "/Game/Blueprints/Treatment/BP_Health.BP_Health_C"))
  (set `self.bNeedTreatment` false)
  (`SceneComponent.SetVisibility` (`self.MedicineWidget`) false false)
  (if Success
    (`/Game/Blueprints/Treatment/BP_Health.AddHP` _returnvalue _damage)
    (else
      (`/Game/Blueprints/Treatment/BP_Health.SubtractHP` _returnvalue _damage))))

(fn `TreatMixture`
  (params (Trimetoprim :type "Float (double-precision)") (Claritromicin :type "Float (double-precision)") (Sulfametoksazol :type "Float (double-precision)"))
  (bind _mixturetreatment (`self.MixtureTreatment`))
  (if (and (== Trimetoprim (`BlueprintMapLibrary.Map_Find` _mixturetreatment "NewEnumerator0")) (== Claritromicin (`BlueprintMapLibrary.Map_Find` _mixturetreatment "NewEnumerator1")) (== Sulfametoksazol (`BlueprintMapLibrary.Map_Find` _mixturetreatment "NewEnumerator2")))
    (`self.Treat` true)
    (else
      (`self.Treat` false))))

(fn `Unpause`
  (`KismetSystemLibrary.K2_UnPauseTimerHandle` (`self.DiseaseTimer`))
  (`KismetSystemLibrary.K2_UnPauseTimerHandle` (`self.DamageTimer`)))