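; BP_CameraSwitch is a trigger actor that changes the camera view when the player enters its box.
; On overlap by a BP_Player component tagged "Capsule", it sets player controller 0's view target to its Camera reference.
; It then passes its stored direction value to the Direction function, which writes it to the player pawn's Direction variable.
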(event `self.Box.OnComponentBeginOverlap`
  (params (OverlappedComponent :type "PrimitiveComponent Object Reference") (OtherActor :type "Actor Object Reference") (OtherComp :type "PrimitiveComponent Object Reference") (OtherBodyIndex :type Integer) (bFromSweep :type Boolean) (SweepResult :type "HitResult Structure (by ref)"))
  (cast `/Game/Blueprints/Character/BP_Player` OtherActor)
  (if (`ActorComponent.ComponentHasTag` OtherComp "Capsule")
    (`PlayerController.SetViewTargetWithBlend` (`GameplayStatics.GetPlayerController` 0) (`self.Camera`) 0.0 "VTBlend_Linear" 0.0 false)
    (`self.Direction` (`self.Directio`))))

(fn `Direction`
  (params (direction :type Integer))
  (bind _asbp_player (cast `/Game/Blueprints/Character/BP_Player` (`GameplayStatics.GetPlayerPawn` 0)))
  (set `/Game/Blueprints/Character/BP_Player.Direction` (`local.direction`) _asbp_player))

(fn `UserConstructionScript`)