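; Actor component that lets its owner interact with nearby actors implementing BPI_Interact, with a WBP_Interact prompt widget.
; A runtime-added sphere tracks overlapping interactables and fades the widget as the list fills or empties.
; InteractFirst messages the first tracked actor, whose reply can pause detection, disable input and show the cursor.
; RestoreInteract restores game input and zeroes then resets the sphere radius to rebuild overlaps.
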(event `self.ReceiveBeginPlay`
  (bind _spherecomponent (`self.SphereComponent`))
  (`|ExecutionSequence`
    (:`then_0`
      (bind _foundwidgets (`WidgetBlueprintLibrary.GetAllWidgetsOfClass` "/Game/Blueprints/Interaction/WBP_Interact.WBP_Interact_C"))
      (if (`KismetArrayLibrary.Array_IsEmpty` _foundwidgets)
        (bind _returnvalue (`|CreateWidget` "/Game/Blueprints/Interaction/WBP_Interact.WBP_Interact_C"))
        (bind _output_get (set `self.InteractWidget` _returnvalue))
        (`Widget.SetRenderOpacity` _output_get 0.0)
        (`UserWidget.AddToViewport` _output_get 0)))
    (:`then_1`
      (bind _returnvalue_2 (`|AddComponentByClass` (`self.GetOwner`) "/Script/Engine.SphereComponent" false (`KismetMathLibrary.MakeTransform` (`self.Offset`))))
      (bind _output_get_2 (set `self.SphereComponent` _returnvalue_2))
      (`SphereComponent.SetSphereRadius` _output_get_2 (`self.Radius`) true)
      (add `PrimitiveComponent.OnComponentBeginOverlap` _spherecomponent (`|CreateDelegate` :!event `BeginOverlap`))
      (add `PrimitiveComponent.OnComponentEndOverlap` _spherecomponent (`|CreateDelegate` :!event `EndOverlap`)))))

(event `BeginOverlap`
  (params (OverlappedComponent :type "PrimitiveComponent Object Reference") (OtherActor :type "Actor Object Reference") (OtherComp :type "PrimitiveComponent Object Reference") (OtherBodyIndex :type Integer) (bFromSweep :type Boolean) (SweepResult :type "HitResult Structure (by ref)"))
  (if (not (`self.Pause`))
    (if (`KismetSystemLibrary.DoesImplementInterface` OtherActor "/Game/Blueprints/Interaction/BPI_Interact.BPI_Interact_C")
      (bind _returnvalue (`KismetArrayLibrary.Array_Add` (`self.InteractedActors`) OtherActor))
      (if (== _returnvalue 0)
        (`/Game/Blueprints/Interaction/WBP_Interact.FadeOut` (`self.InteractWidget`))))))

(event `EndOverlap`
  (params (OverlappedComponent :type "PrimitiveComponent Object Reference") (OtherActor :type "Actor Object Reference") (OtherComp :type "PrimitiveComponent Object Reference") (OtherBodyIndex :type Integer))
  (if (`KismetArrayLibrary.Array_Contains` (`self.InteractedActors`) OtherActor)
    (`KismetArrayLibrary.Array_RemoveItem` (`self.InteractedActors`) OtherActor)
    (if (== (`KismetArrayLibrary.Array_Length` (`self.InteractedActors`)) 0)
      (`/Game/Blueprints/Interaction/WBP_Interact.FadeIn` (`self.InteractWidget`)))))

(fn `InteractFirst`
  (bind _returnvalue (`GameplayStatics.GetPlayerController` 0))
  (bind _output (`|GetArrayItem` (`self.InteractedActors`)))
  (if (`KismetSystemLibrary.DoesImplementInterface` _output "/Game/Blueprints/Interaction/BPI_Interact.BPI_Interact_C")
    (bind (_stopinteraction _disableinput _showcursor) (message `/Game/Blueprints/Interaction/BPI_Interact.Interact` _output self))
    (`|ExecutionSequence`
      (:`then_0`
        (bind _output_get (set `self.Pause` _stopinteraction))
        (if _output_get
          (`/Game/Blueprints/Interaction/WBP_Interact.FadeIn` (`self.InteractWidget`))))
      (:`then_1`
        (if _disableinput
          (`Actor.DisableInput` (`self.GetOwner`) _returnvalue)))
      (:`then_2`
        (set `PlayerController.bShowMouseCursor` _showcursor _returnvalue)
        (`WidgetBlueprintLibrary.SetInputMode_GameAndUIEx` _returnvalue null "DoNotLock" false)))))

(fn `RestoreInteract`
  (bind _returnvalue (`GameplayStatics.GetPlayerController` 0))
  (set `self.Pause` false)
  (`KismetArrayLibrary.Array_Clear` (`self.InteractedActors`))
  (`SphereComponent.SetSphereRadius` (`self.SphereComponent`) 0.0 true)
  (`SphereComponent.SetSphereRadius` (`self.SphereComponent`) (`self.Radius`) true)
  (`Actor.EnableInput` (`self.GetOwner`) (`GameplayStatics.GetPlayerController` 0))
  (`WidgetBlueprintLibrary.SetInputMode_GameOnly` _returnvalue)
  (set `PlayerController.bShowMouseCursor` false _returnvalue))